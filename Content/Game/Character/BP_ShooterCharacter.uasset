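; BP_ShooterCharacter is the shooter character Blueprint, which here handles the aim-down camera zoom.
; AimingSwitch plays or reverses the SocketCameraOffset timeline, whose value scales the spring arm socket offset on all three axes.
; While aiming, each update cumulatively subtracts from the camera FOV.
; When aim is released, it lerps between the FOV captured at aim start and the current one.
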(event EventAimingSwitch
  (params (aim :type Boolean))
  (bind _followcamera (Variables|Default|GetFollowCamera))
  (bind _fieldofview (Variables|/Script/Engine.CameraComponent|GetFieldOfView _followcamera))
  ;[1 1 1] Zooming Aim
  (if aim
    (bind _output_get (Variables|Default|SetStartFOV (Variables|/Script/Engine.CameraComponent|GetFieldOfView (Variables|Default|GetFollowCamera))))
    (bind _socket_offset (Timeline|Socket%20Camera%20Offset Play)
      (:Update
        (Variables|/Script/Engine.SpringArmComponent|SetSocketOffset (Variables|Default|GetCameraSpring) (Math|Vector|MakeVector (* _socket_offset 2e+02) (/ (* _socket_offset 2e+02) 1.25) (/ (* _socket_offset 2e+02) 2.5)))
        (if aim
          (Camera|SetFieldOfView _followcamera (- _fieldofview (* 4 _socket_offset)))
          (else
            (Camera|SetFieldOfView (Variables|Default|GetFollowCamera) (Math|Float|Lerp _output_get _fieldofview (* 3 _socket_offset)))))))
    (else
      (Timeline|Socket%20Camera%20Offset Reverse))))

(fn ConstructionScript)